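; Player character that switches between first- and third-person views and fires projectiles.
; On BeginPlay it binds inherited perspective and shoot events, which reattach the camera to capsule or boom, hide the mesh in first person, and spawn BP_Projectile at Firepoint.
; Tick prints a debug message showing whether the actor in front of the camera implements CC_Interactable.
; GetDesiredHandLocation line-traces from the camera for an aim point, returning zero on a miss.
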(event Custom|m_OnPerspectiveChanged_Event
  (params (_ToPerspective :type EPlayerPerspective%20Enum :default "FirstPerson"))
  ;[1 1 1] Bind To Perspective Changed
  (Utilities|FlowControl|Sequence
    (:then_0
      (switch Utilities|FlowControl|Switch|SwitchonEPlayerPerspective _ToPerspective
        (:FirstPerson
          (Transformation|AttachComponentToComponent (Variables|Default|Getm_Camera) (Variables|Default|GetCapsuleComponent) "None" "SnapToTarget" "SnapToTarget" "KeepRelative" true)
          (Transformation|SetRelativeLocation (Variables|Default|Getm_Camera) (Variables|Default|Getm_CameraOffset) false false))
        (:ThirdPerson
          (Transformation|AttachComponentToComponent (Variables|Default|Getm_Camera) (Variables|Default|Getm_CameraBoom) "None" "SnapToTarget" "SnapToTarget" "KeepRelative" true))))
    (:then_1
      ;[1 1 1] Hide Mesh in First Person
      (Development|SetHiddeninGame (Variables|Character|GetMesh) (Utilities|Enum|Equal(Enum) _ToPerspective "FirstPerson") false))))

(event Custom|BP%20Shooting
  (bind _firepoint (Variables|Default|GetFirepoint))
  ;[1 1 1] Add Shooting Function
  (bind _returnvalue (Game|SpawnActorfromClass "/Game/Blueprints/BP_Projectile.BP_Projectile_C" (Math|Transform|MakeTransform (Transformation|GetWorldLocation _firepoint) (Transformation|GetWorldRotation _firepoint) "1.000000,1.000000,1.000000") "Undefined" "MultiplyWithRoot" 0 0))
  (if (Utilities|IsValid (Actor|GetComponentbyClass _returnvalue "/Script/Engine.ProjectileMovementComponent"))
    _))

(event EventBeginPlay
  (Utilities|FlowControl|Sequence
    (:then_0
      ;[1 1 1] Bind To Perspective Changed
      (EventDispatchers|BindEventtoMonPerspectiveChanged (delegate Custom|m_OnPerspectiveChanged_Event)))
    (:then_1
      ;[1 1 1] Add Shooting Function
      (EventDispatchers|BindEventtoMonShoot (delegate Custom|BP%20Shooting)))))

(event Collision|EventActorBeginOverlap
  (params (OtherActor :type Actor%20Object%20Reference)))

(event EventTick
  (params (DeltaSeconds :type Float%20%28single-precision%29))
  (Utilities|FlowControl|Sequence
    (:then_0
      ;[1 1 1] Looking at interactable ?
      (bind _returnvalue (Class|CCCharacter|GetActorinFronOfCamera))
      (if (and (Utilities|IsValid _returnvalue) (Utilities|DoesObjectImplementInterface _returnvalue "/Script/CrystalClear.CC_Interactable"))
        (Development|PrintString (Utilities|String|Append "Hit : " (Utilities|GetDisplayName _returnvalue)) true true "(R=0.016853,G=1.000000,B=0.000000,A=1.000000)" 5.0 "INTERACT_LOOKUP")
        (else
          (Development|PrintString (Utilities|String|Append "Hit : " "Nothing") true true "(R=1.000000,G=0.014804,B=0.000000,A=1.000000)" 5.0 "INTERACT_LOOKUP"))))))

(fn ConstructionScript)

(fn GetDesiredHandLocation
  (bind _m_camera (Variables|Default|Getm_Camera))
  (bind _returnvalue (Transformation|GetWorldLocation _m_camera))
  (bind (_outhit _returnvalue_2) (Collision|LineTraceByChannel _returnvalue (+ _returnvalue (* (Math|Vector|GetForwardVector _m_camera) 1e+04)) "TraceTypeQuery1" false 0 "None"))
  (if _returnvalue_2
    (return (.Location (Collision|BreakHitResult _outhit)))
    (else
      (return "0, 0, 0"))))