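; Player controller that owns the main HUD and switches between gameplay and UI input modes.
; SpawnHUD creates the MainHUD widget, adds it to the viewport, shares it with the Player_BP pawn and immediately calls its OpenInventory.
; A separate OpenInventory event forwards to the HUD.
; SetGameInput and SetUIInput toggle the input mode and mouse cursor, with UI mode focusing the HUD.
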(event EventBeginPlay)

(event EventTick
  (params (DeltaSeconds :type Float%20%28single-precision%29)))

(event EventSpawnHUD
  (bind _asplayer_bp (Utilities|Casting|CastToPlayer_BP (Game|Player|GetPlayerPawn 0)))
  (bind _output_get (Variables|Default|SetPlayerBP _asplayer_bp))
  (bind _returnvalue (UserInterface|CreateWidget "/Game/HUD/MainHUd.MainHUD_C" 0 _output_get))
  (bind _output_get_2 (Variables|Default|SetMainHUD _returnvalue))
  (UserInterface|Viewport|AddtoViewport _output_get_2 0)
  (Variables|/Game/Blueprints/Player_BP.Player_BP_C|SetMainHUD _asplayer_bp _output_get_2)
  (Default|OpenInventory _output_get_2))

(event EventOpenInventory
  (Default|OpenInventory (Variables|Default|GetMainHUD)))

(fn ConstructionScript)

(fn SetGameInput
  (Input|SetInputModeGameOnly self)
  (Variables|Default|SetbShowMouseCursor false))

(fn SetUIInput
  (Input|SetInputModeGameandUI self (Variables|Default|GetMainHUD) "LockOnCapture" true)
  (Variables|Default|SetbShowMouseCursor true))